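; BP_Key is a key pickup that responds to an Interact event, notifying its Door reference and setting HasKey.
; It shows a WBP_KeyPopUp widget and immediately hides its cube mesh and disables that mesh's collision.
; After a short delay it removes the popup, adds a key icon widget to the viewport and destroys itself.
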(event `/Game/Blueprint/BPI_Interact.Interact`
  (bind _returnvalue (`GameplayStatics.GetPlayerController` 0))
  (bind _cube (`self.Cube`))
  (message `/Game/Blueprint/BPI_Door.PickUp key` (`self.Door`))
  (bind _returnvalue_2 (`|CreateWidget` "/Game/PickUp/WBP_KeyPopUp.WBP_KeyPopUp_C" _returnvalue))
  (bind _output_get (set `self.KeyPopUp` _returnvalue_2))
  (`UserWidget.AddToViewport` _output_get 0)
  (set `self.HasKey?` true)
  (`|ExecutionSequence`
    (:`then_0`
      (`SceneComponent.SetVisibility` _cube false false)
      (`PrimitiveComponent.SetCollisionEnabled` _cube "NoCollision"))
    (:`then_1`
      (`KismetSystemLibrary.Delay` 3.0)
      (`Widget.RemoveFromParent` _returnvalue_2)
      (bind _returnvalue_3 (`|CreateWidget` "/Game/PickUp/WBP_KeyIcon.WBP_KeyIcon_C" _returnvalue))
      (`UserWidget.AddToViewport` _returnvalue_3 0)
      (`self.K2_DestroyActor`))))

(fn `UserConstructionScript`)