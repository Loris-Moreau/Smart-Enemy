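; BP_Door is a key-locked door that swings open and closed on interaction.
; The PickUpKey event sets HasKey, and Interact does nothing without it.
; With the key, a FlipFlop alternates between playing and reversing DoorTimeline, printing debug strings along the way.
; The timeline track lerps the yaw of the Billboard component up to 110 degrees, which apparently serves as the hinge pivot.
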(event `/Game/Blueprint/BPI_Interact.Interact`
  (if (`self.HasKey?`)
    (`KismetSystemLibrary.PrintString` "true")
    (`/Engine/EditorBlueprintResources/StandardMacros.FlipFlop`
      (:`A`
        (`KismetSystemLibrary.PrintString` "ça ouvre")
        (bind (_direction _door_track) (`Timeline|Door Timeline` :!label _label)
          (:`Update`
            (`SceneComponent.K2_SetRelativeRotation` (`self.Billboard`) (`KismetMathLibrary.MakeRotator` 0.0 0.0 (`KismetMathLibrary.Lerp` 0.0 110.0 _door_track)) false false))))
      (:`B`
        (`KismetSystemLibrary.PrintString` "ça ferme")
        (goto _label :!via `Reverse`)))))

(event `/Game/Blueprint/BPI_Door.PickUp key`
  (set `self.HasKey?` true))

(fn `UserConstructionScript`)