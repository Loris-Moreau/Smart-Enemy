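; Base enemy character Blueprint that supplies a melee attack and movement data, likely for AI logic to drive.
; Attack plays a punch montage, applies fixed damage to the player on completion without a range check, and prints the result.
; Completion or interruption fires the OnAttackEnd dispatcher.
; Getters expose the patrol route and attack and strafe radii, while SetMovementSpeed maps a speed state to max walk speed.
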(event `self.ReceiveBeginPlay`)

(event `Attack`
  (`|PlayMontage` (`self.Mesh`) "/Game/Characters/Enemy/Animation/Cross_Punch_Montage.Cross_Punch_Montage"
    (:`OnCompleted`
      (bind _returnvalue (`GameplayStatics.ApplyDamage` (`GameplayStatics.GetPlayerCharacter` 0) 10.0 null self "/Script/Engine.DamageType"))
      (`KismetSystemLibrary.PrintString` (`KismetStringLibrary.Conv_DoubleToString` _returnvalue) true false (struct :`R` 1.0 :`B` 0.075629 :`A` 1.0)))
    (:`OnInterrupted`
      _))
  (`self.OnAttackEnd`))

(fn `Get Patrol Route`
  (returns (`Patrol Route` :type "/Game/Characters/Enemy/Behaviour/BP_Patrol_Route Object Reference"))
  (return (`self.Patrol Route`)))

(fn `GetIdealRange`
  (returns (AttackRadius :type "Float (double-precision)") (StrafeRadius :type "Float (double-precision)"))
  (return 20.0 350.0))

(fn `SetMovementSpeed`
  (params (Speeds :type "/Game/Characters/Enemy/Behaviour/Enums/E_Movement_Speeds Enum" :default "NewEnumerator5"))
  (returns (`Speed Value` :type "Float (double-precision)"))
  (bind _output_get (set `CharacterMovementComponent.MaxWalkSpeed` (select `/Game/Characters/Enemy/Behaviour/Enums/E_Movement_Speeds` Speeds :`NewEnumerator0` 220.0 :`NewEnumerator4` 270.0 :`NewEnumerator1` 350.0 :!type "Float (single-precision)") (`self.CharacterMovement`)))
  (return _output_get))

(fn `UserConstructionScript`)